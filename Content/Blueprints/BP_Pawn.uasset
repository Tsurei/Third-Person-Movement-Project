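; BP_Pawn is a player pawn with camera-relative movement and mouse look through Enhanced Input, adding its movement mapping context on BeginPlay.
; Mouse input drives controller yaw and pitch.
; Move input is projected onto the spring arm's flattened forward and right vectors, clamped in length and applied as an unswept local offset, without delta-time scaling.
; Tick prints the spring arm rotation and forward vector for debugging.
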(event `self.ReceiveBeginPlay`
  (bind _asplayer_controller (cast `PlayerController` (`self.GetController`)))
  (`EnhancedInputSubsystemInterface.AddMappingContext` (pcsubsystem `EnhancedInputLocalPlayerSubsystem` _asplayer_controller) "/Game/Input/IMC_Movement.IMC_Movement" 0 (struct)))

(event `EnhancedInput|/Game/Input/IA_Move`
  (params (ActionValue :type "Vector2D Structure") (ElapsedSeconds :type "Float (double-precision)") (TriggeredSeconds :type "Float (double-precision)") (InputAction :type "InputAction Object Reference" :default "/Game/Input/IA_Move.IA_Move"))
  (bind _returnvalue (`SpringArmComponent.GetTargetRotation` (`self.SpringArm`)))
  (bind (_returnvalue_x _returnvalue_y) (`KismetMathLibrary.BreakVector` (`KismetMathLibrary.GetForwardVector` _returnvalue)))
  (bind (_returnvalue_x_2 _returnvalue_y_2) (`KismetMathLibrary.BreakVector` (`KismetMathLibrary.GetRightVector` _returnvalue)))
  ; Character Movement
  (:`Triggered`
    (`self.K2_AddActorLocalOffset` (`KismetMathLibrary.ClampVectorSize` (* (+ (* ActionValue_X (`KismetMathLibrary.MakeVector` _returnvalue_x _returnvalue_y)) (* ActionValue_Y (`KismetMathLibrary.MakeVector` _returnvalue_x_2 _returnvalue_y_2))) 10.0) 3.0 20.0))))

(event `EnhancedInput|/Game/Input/IA_Mouse`
  (params (ActionValue :type "Vector2D Structure") (ElapsedSeconds :type "Float (double-precision)") (TriggeredSeconds :type "Float (double-precision)") (InputAction :type "InputAction Object Reference" :default "/Game/Input/IA_Mouse.IA_Mouse"))
  ; Camera Control
  (:`Triggered`
    (`self.AddControllerYawInput` ActionValue_X)
    (`self.AddControllerPitchInput` ActionValue_Y)))

(event `self.ReceiveTick`
  (params (DeltaSeconds :type "Float (single-precision)"))
  (bind _returnvalue (`SpringArmComponent.GetTargetRotation` (`self.SpringArm`)))
  (`KismetSystemLibrary.PrintString` (`KismetStringLibrary.Concat_StrStr` (`KismetStringLibrary.Conv_RotatorToString` _returnvalue) (`KismetStringLibrary.Concat_StrStr` " \nForward Vector" (`KismetStringLibrary.Conv_VectorToString` (`KismetMathLibrary.GetForwardVector` _returnvalue)))) true true (struct :`R` 0.234047 :`G` 1.0 :`B` 0.043859 :`A` 1.0) 2.0 "Spring Rotation"))

(fn `UserConstructionScript`)