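; BP_CharacterController is a player controller that turns Enhanced Input actions into movement commands for the possessed BP_Pawn.
; On BeginPlay it adds the IMC_Movement mapping context and caches the controlled pawn, cast to BP_Pawn.
; Move and mouse actions pass their values through, jump, slide and sprint set on/off states on press and release, and dash fires on trigger.
; All movement logic is left to the pawn.
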(event `self.ReceiveBeginPlay`
  (`EnhancedInputSubsystemInterface.AddMappingContext` (pcsubsystem `EnhancedInputLocalPlayerSubsystem` (`GameplayStatics.GetPlayerControllerFromID` (`GameplayStatics.GetPlayerControllerID` self))) "/Game/Input/IMC_Movement.IMC_Movement" 0 (struct))
  (bind _asbp_pawn (cast `/Game/Blueprints/BP_Pawn` (`self.K2_GetPawn`)))
  (set `self.ControlledPawn` _asbp_pawn))

(event `EnhancedInput|/Game/Input/IA_Move`
  (params (ActionValue :type "Vector2D Structure") (ElapsedSeconds :type "Float (double-precision)") (TriggeredSeconds :type "Float (double-precision)") (InputAction :type "InputAction Object Reference" :default "/Game/Input/IA_Move.IA_Move"))
  (:`Triggered`
    (`/Game/Blueprints/BP_Pawn.SetMoveInput` (`self.ControlledPawn`) ActionValue)))

(event `EnhancedInput|/Game/Input/IA_Mouse`
  (params (ActionValue :type "Vector2D Structure") (ElapsedSeconds :type "Float (double-precision)") (TriggeredSeconds :type "Float (double-precision)") (InputAction :type "InputAction Object Reference" :default "/Game/Input/IA_Mouse.IA_Mouse"))
  (:`Triggered`
    (`/Game/Blueprints/BP_Pawn.SetLookInput` (`self.ControlledPawn`) ActionValue)))

(event `EnhancedInput|/Game/Input/IA_Jump`
  (params (ActionValue :type "Float (double-precision)") (ElapsedSeconds :type "Float (double-precision)") (TriggeredSeconds :type "Float (double-precision)") (InputAction :type "InputAction Object Reference" :default "/Game/Input/IA_Jump.IA_Jump"))
  (bind _controlledpawn (`self.ControlledPawn`))
  (:`Started`
    (`/Game/Blueprints/BP_Pawn.SetJump` _controlledpawn true))
  (:`Completed`
    (`/Game/Blueprints/BP_Pawn.SetJump` _controlledpawn false)))

(event `EnhancedInput|/Game/Input/IA_Dash`
  (params (ActionValue :type Boolean) (ElapsedSeconds :type "Float (double-precision)") (TriggeredSeconds :type "Float (double-precision)") (InputAction :type "InputAction Object Reference" :default "/Game/Input/IA_Dash.IA_Dash"))
  (:`Triggered`
    (`/Game/Blueprints/BP_Pawn.TriggerDash` (`self.ControlledPawn`))))

(event `EnhancedInput|/Game/Input/IA_Slide`
  (params (ActionValue :type Boolean) (ElapsedSeconds :type "Float (double-precision)") (TriggeredSeconds :type "Float (double-precision)") (InputAction :type "InputAction Object Reference" :default "/Game/Input/IA_Slide.IA_Slide"))
  (bind _controlledpawn (`self.ControlledPawn`))
  (:`Started`
    (`/Game/Blueprints/BP_Pawn.SetSlide` _controlledpawn true))
  (:`Completed`
    (`/Game/Blueprints/BP_Pawn.SetSlide` _controlledpawn false)))

(event `EnhancedInput|/Game/Input/IA_Sprint`
  (params (ActionValue :type Boolean) (ElapsedSeconds :type "Float (double-precision)") (TriggeredSeconds :type "Float (double-precision)") (InputAction :type "InputAction Object Reference" :default "/Game/Input/IA_Sprint.IA_Sprint"))
  (bind _controlledpawn (`self.ControlledPawn`))
  (:`Started`
    (`/Game/Blueprints/BP_Pawn.SetSprint` _controlledpawn true))
  (:`Completed`
    (`/Game/Blueprints/BP_Pawn.SetSprint` _controlledpawn false)))

(fn `UserConstructionScript`)